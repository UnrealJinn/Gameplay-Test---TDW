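; GA_LeapSlam is a GAS ability that launches the character into a leap and damages pawns around the landing point.
; On commit, a root motion jump force runs for the character's attack duration, deriving direction and clamped height from the avatar's scaled location.
; Landing fires the slam cue and applies SetByCaller damage to overlapped actors with an ability system, excluding the caster.
; Finishing commits the cooldown and ends the ability.
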(event Ability|EventActivateAbility
  (bind _returnvalue (Ability|GetAvatarActorfromActorInfo))
  (bind _asbp_arpgcharacter (Utilities|Casting|CastToBP_ARPGCharacter _returnvalue))
  (bind _returnvalue_2 (Transformation|GetActorLocation _asbp_arpgcharacter))
  (bind _returnvalue_3 (* _returnvalue_2 5e+02))
  (bind _returnvalue_4 (Ability|CommitAbility))
  (if _returnvalue_4
    (Utilities|Array|AddUnique (Variables|Default|GetActors%20to%20Ignore) _asbp_arpgcharacter)
    (|ApplyRootMotionJumpForce "None" (Math|Rotator|FindLookatRotation _returnvalue_2 _returnvalue_3) 0.0 (Math|Float|Clamp(Float) (* (Math|Vector|Distance(Vector) _returnvalue_2 _returnvalue_3) 0.35) 3e+02 8e+02) (Default|CalculateAttackDuration _asbp_arpgcharacter) 0.1 true "MaintainLastRootMotionVelocity" "0, 0, 0" 0.0
      (:OnFinish
        (Ability|CommitAbilityCooldown false)
        (Ability|EndAbility))
      (:OnLanded
        (GameplayCue|ExecuteGameplayCue :GameplayCueTag "(TagName=\"GameplayCue.Slam.Active\")")
        (bind _outactors (Collision|SphereOverlapActors _returnvalue_2 5e+02 (Variables|Default|GetObject%20Types) "/Script/Engine.Pawn" (Variables|Default|GetActors%20to%20Ignore)))
        (for _array_element _outactors
          (Utilities|IsValid (Ability|GetAbilitySystemComponent _array_element)
            (:Is%20Valid
              (bind _returnvalue_5 (Spec|MakeSpecHandle(ByClass) "/Game/ARPG/GAS/Effects/GE_Health_Damage.GE_Health_Damage_C" 0 (.AsBP%20ARPGCharacter (Utilities|Casting|CastToBP_ARPGCharacter (Ability|GetAvatarActorfromActorInfo)))))
              (bind _returnvalue_6 (Ability|GameplayEffect|AssignTagSetbyCallerMagnitude _returnvalue_5 "(TagName=\"Data.Damage\")" -25.0))
              (GameplayEffects|ApplyGameplayEffectSpecToSelf (Ability|GetAbilitySystemComponent _array_element) _returnvalue_6))))))
    (else
      (Ability|EndAbility))))

(event Ability|EventOnEndAbility
  (params (bWasCancelled :type Boolean)))